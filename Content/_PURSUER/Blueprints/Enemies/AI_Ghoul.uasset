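; AI controller for the Ghoul enemy that wanders the navmesh until perception flags the player, then chases.
; Wander loops random nearby moves with pauses after each success; a failed move ends the loop.
; Once IsSensed is set, the next Wander starts a looping timer that re-issues a move to the player.
; Both perception branches set IsSensed true, so losing the player never returns it to wandering.
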(event OnTargetPerceptionUpdated(AIPerception)
  (params (Actor :type Actor%20Object%20Reference) (Stimulus :type AI%20Stimulus%20Structure))
  (Utilities|Casting|CastToBP_PlayerCharacter Actor)
  (if (.bSuccessfullySensed (Utilities|Struct|BreakAIStimulus Stimulus))
    (Variables|Default|SetisSensed true)
    (else
      (Variables|Default|SetisSensed true)))
  (Development|PrintString (Utilities|String|ToString(Boolean) (Variables|Default|GetisSensed))))

(event Custom|Wander
  (if (Variables|Default|GetisSensed)
    (Utilities|Time|SetTimerbyFunctionName 0 "Chase" 0.5 true)
    (else
      (AI|AIMoveTo (Pawn|GetControlledPawn) (.RandomLocation (Class|NavigationSystemV1|GetRandomPointinNavigableRadius (Transformation|GetActorLocation (Pawn|GetControlledPawn)) 1e+03 0 0)) 0 5.0 false
        (:OnSuccess
          (Utilities|FlowControl|Delay (Math|Random|RandomFloatinRange 1.0 3.0))
          (CallFunction|Wander))))))

(event Custom|Chase
  (if (Variables|Default|GetisSensed)
    (AI|AIMoveTo (Pawn|GetControlledPawn) "0, 0, 0" (Game|GetPlayerCharacter 0) 5.0 false)
    (else
      (Utilities|Time|ClearTimerbyFunctionName 0 "Chase")
      (CallFunction|Wander))))

(event EventBeginPlay
  (CallFunction|Wander))

(fn ConstructionScript)