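; BP_Spider is a spider enemy that hurts whatever it touches.
; It plays a chattering sound at its location when play begins, after running the parent's BeginPlay logic.
; Any capsule overlap sends the other actor a fixed, non-critical TakeDamage message and plays a creature sound, with no filtering in this Blueprint.
; Its destruction only prints a debug string.
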(event OnComponentBeginOverlap(Capsule)
  (params (OverlappedComponent :type Primitive%20Component%20Object%20Reference) (OtherActor :type Actor%20Object%20Reference) (OtherComp :type Primitive%20Component%20Object%20Reference) (OtherBodyIndex :type Integer) (bFromSweep :type Boolean) (SweepResult :type Hit%20Result%20Structure%20%28by%20ref%29))
  ;[1 1 1] Whenever collides with a damageable entity, cause damage to that entity
  (Class|BPIDamageable|TakeDamage(Message) OtherActor 2e+01 false 0.0)
  (Audio|PlaySoundatLocation "/Game/FirstPerson/Audio/tiny-vicious-creature-47253.tiny-vicious-creature-47253" (Transformation|GetActorLocation) "0, 0, 0" 1.0 1.0 0.0 0 0 0))

(event EventBeginPlay
  (|CallParentFunction)
  (Audio|PlaySoundatLocation "/Game/FirstPerson/Audio/spider-chattering-87558_Cue.spider-chattering-87558_Cue" (Transformation|GetActorLocation) "0, 0, 0" 1.0 1.0 0.0 0 0 0))

(event EventOnDestroy
  (Development|PrintString "A spider has been destroyed"))

(fn ConstructionScript
  (|CallParentFunction))