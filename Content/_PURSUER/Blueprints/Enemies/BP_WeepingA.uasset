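; Weeping Angel-style enemy character that pursues the first-person player only while off screen.
; When PawnSensing sees the player, it projects its own location to screen space and tests it against the viewport bounds.
; On screen it stops movement immediately, otherwise it calls AIMoveTo toward the player, with no occlusion check.
; Mesh overlap with the player applies fixed damage.
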(event OnSeePawn(PawnSensing)
  (params (Pawn :type Pawn%20Object%20Reference))
  (bind _returnvalue (Transformation|GetActorLocation))
  (bind _returnvalue_2 (Game|GetPlayerController 0))
  (bind _returnvalue_3 (Viewport|GetViewportSize))
  (bind _screenlocation (Class|PlayerController|ProjectWorldLocationtoScreen _returnvalue_2 _returnvalue false))
  (bind _asfirst_person_character (Utilities|Casting|CastToFirstPersonCharacter Pawn))
  (if (Math|Boolean|ANDBoolean (> (.x _screenlocation) 0.0) (> (.y _screenlocation) 0.0) (< (.x _screenlocation) (.x _returnvalue_3)) (< (.y _screenlocation) (.y _returnvalue_3)))
    (Components|Movement|StopMovementImmediately (Variables|Character|GetCharacterMovement))
    (else
      (AI|AIMoveTo self "0, 0, 0" _asfirst_person_character 5.0 false))))

(event OnComponentBeginOverlap(Mesh)
  (params (OverlappedComponent :type Primitive%20Component%20Object%20Reference) (OtherActor :type Actor%20Object%20Reference) (OtherComp :type Primitive%20Component%20Object%20Reference) (OtherBodyIndex :type Integer) (bFromSweep :type Boolean) (SweepResult :type Hit%20Result%20Structure%20%28by%20ref%29))
  (bind _asfirst_person_character (Utilities|Casting|CastToFirstPersonCharacter OtherActor))
  (Game|Damage|ApplyDamage _asfirst_person_character 2e+01 0 0))

(event EventBeginPlay)

(event Collision|EventActorBeginOverlap
  (params (OtherActor :type Actor%20Object%20Reference)))

(event EventTick
  (params (DeltaSeconds :type Float%20%28single-precision%29)))

(fn ConstructionScript)