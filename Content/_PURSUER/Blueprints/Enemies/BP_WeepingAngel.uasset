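; BP_WeepingAngel is an enemy that advances on the player only while it is off-screen, damaging actors its cube overlaps.
; When PawnSensing sees the player, it projects the cube's location to screen space, stopping immediately if within viewport bounds, otherwise issuing AI MoveTo.
; A sphere trigger tracks player proximity: moving while close swaps the image to a hunt material, and leaving restores the ambient one.
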(event OnSeePawn(PawnSensing)
  (params (Pawn :type Pawn%20Object%20Reference))
  (bind _returnvalue (Game|GetPlayerController 0))
  (bind _returnvalue_2 (Viewport|GetViewportSize))
  (bind _cube (Variables|Default|GetCube))
  (bind _returnvalue_3 (Transformation|GetWorldLocation _cube))
  (bind _screenlocation (Class|PlayerController|ProjectWorldLocationtoScreen _returnvalue _returnvalue_3 false))
  ;[1 1 1] When the weeping angel sees the player, check if it is in player's view. If not, move towards them. ()
  (bind _asbp_player_character (Utilities|Casting|CastToBP_PlayerCharacter Pawn))
  (if (Math|Boolean|ANDBoolean (> (.x _screenlocation) 0.0) (> (.y _screenlocation) 0.0) (< (.x _screenlocation) (.x _returnvalue_2)) (< (.y _screenlocation) (.y _returnvalue_2)))
    (Components|Movement|StopMovementImmediately (Variables|Character|GetCharacterMovement))
    (else
      (AI|AIMoveTo self "0, 0, 0" _asbp_player_character 2.0 false
        (:then
          (if (Variables|Default|GetClose)
            (Rendering|Material|SetMaterial (Variables|Default|GetImage) 0 "/Game/_PURSUER/Blueprints/Enemies/WEEP_HUNT.WEEP_HUNT")))))))

(event OnComponentBeginOverlap(Cube)
  (params (OverlappedComponent :type Primitive%20Component%20Object%20Reference) (OtherActor :type Actor%20Object%20Reference) (OtherComp :type Primitive%20Component%20Object%20Reference) (OtherBodyIndex :type Integer) (bFromSweep :type Boolean) (SweepResult :type Hit%20Result%20Structure%20%28by%20ref%29))
  ;[1 1 1] Whenever collides with a damageable entity, cause damage to that entity
  (Class|BPIDamageable|TakeDamage(Message) OtherActor 2e+01 false 0.0))

(event OnComponentEndOverlap(Sphere)
  (params (OverlappedComponent :type Primitive%20Component%20Object%20Reference) (OtherActor :type Actor%20Object%20Reference) (OtherComp :type Primitive%20Component%20Object%20Reference) (OtherBodyIndex :type Integer))
  (Utilities|Casting|CastToBP_PlayerCharacter OtherActor)
  (Rendering|Material|SetMaterial (Variables|Default|GetImage) 0 "/Game/_PURSUER/Blueprints/Enemies/WEEP_ambient.WEEP_ambient")
  (Variables|Default|SetClose false))

(event OnComponentBeginOverlap(Sphere)
  (params (OverlappedComponent :type Primitive%20Component%20Object%20Reference) (OtherActor :type Actor%20Object%20Reference) (OtherComp :type Primitive%20Component%20Object%20Reference) (OtherBodyIndex :type Integer) (bFromSweep :type Boolean) (SweepResult :type Hit%20Result%20Structure%20%28by%20ref%29))
  (Utilities|Casting|CastToBP_PlayerCharacter OtherActor)
  (Variables|Default|SetClose true))

(fn ConstructionScript)