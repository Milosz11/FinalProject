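; Base Blueprint class for enemies that tracks health and handles incoming damage.
; BeginPlay sets current health to max, and Damage subtracts the received amount, scaled by a critical factor on critical hits.
; When health drops to zero or below it calls OnDestroy, left empty for child classes to implement their own destruction.
; A Heal event exists but is not implemented.
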(event EventBeginPlay
  ;[1 1 1] Event BeginPlay
  (Variables|Default|SetCurrentHealth (Variables|Default|GetMaxHealth)))

(event EventHeal
  (params (healingReceived :type Float%20%28single-precision%29) (isCriticalHit? :type Boolean) (criticalHitFactor :type Float%20%28single-precision%29))
  ;[1 1 1] Currently not handling healing for enemy types
)

(event EventDamage
  (params (damageReceived :type Float%20%28single-precision%29) (isCriticalHit? :type Boolean) (criticalHitFactor :type Float%20%28single-precision%29))
  ;[1 1 1] On damage, subtract health and destroy if below zero
  (bind _output_get (Variables|Default|SetCurrentHealth (- (Variables|Default|GetCurrentHealth) (Math|Float|SelectFloat (* damageReceived criticalHitFactor) damageReceived isCriticalHit?))))
  (if (<= _output_get 0.0)
    (CallFunction|OnDestroy)))

(event EventOnDestroy
  ;[1 1 1] We let child classes implement how they should be destroyed
)

(fn ConstructionScript)