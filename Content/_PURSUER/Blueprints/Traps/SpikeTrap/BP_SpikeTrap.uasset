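; Spike trap that raises its spikes when triggered and damages actors that overlap them.
; TriggerTrap starts a timeline that lerps the spike mesh between start and end locations, while a timer reverses it after the reset time.
; A DoOnce in the timeline update, reset on finish, plays the 2D spike sound once per completed movement.
; Spike overlaps send a damage message with the trap's damage and critical-hit settings.
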(event OnComponentBeginOverlap(SpikesMesh)
  (params (OverlappedComponent :type Primitive%20Component%20Object%20Reference) (OtherActor :type Actor%20Object%20Reference) (OtherComp :type Primitive%20Component%20Object%20Reference) (OtherBodyIndex :type Integer) (bFromSweep :type Boolean) (SweepResult :type Hit%20Result%20Structure%20%28by%20ref%29))
  ;[1 1 1] If any damageable actor overlaps with the spikes, cause damage
  (Class|BPIDamageable|TakeDamage(Message) OtherActor (Variables|Default|GetTrapDamage) (Variables|Default|GetTrapIsCriticalHit) (Variables|Default|GetTrapCriticalHitFactor)))

(event Custom|StartTimeline
  ;[1 1 1] Moves the spike trap up, then after "Time to Reset Trap", moves the spike trap back down, plays spike audio
  (Utilities|Time|SetTimerbyEvent (delegate Custom|ReverseTimeline) (Variables|Default|GetTimeToResetTrap))
  (bind _spike_trap_curve (Timeline|Spike%20Trap%20Timeline Play)
    (:Update
      (Transformation|SetRelativeLocation (Variables|Default|GetSpikesMesh) (Math|Vector|Lerp(Vector) (Variables|Default|GetStartLocation) (Variables|Default|GetEndLocation) _spike_trap_curve) false false)
      (Utilities|FlowControl|DoOnce false :!label _label
        (:Completed
          (Audio|PlaySound2D "/Game/FirstPerson/Audio/SpikeTrapAudio.SpikeTrapAudio" 1.0 1.0 0.0 0 0))))
    (:Finished
      (goto _label Reset))))

(event Custom|ReverseTimeline
  ;[1 1 1] Moves the spike trap up, then after "Time to Reset Trap", moves the spike trap back down, plays spike audio
  (bind _spike_trap_curve (Timeline|Spike%20Trap%20Timeline Reverse)
    (:Update
      (Transformation|SetRelativeLocation (Variables|Default|GetSpikesMesh) (Math|Vector|Lerp(Vector) (Variables|Default|GetStartLocation) (Variables|Default|GetEndLocation) _spike_trap_curve) false false)
      (Utilities|FlowControl|DoOnce false :!label _label
        (:Completed
          (Audio|PlaySound2D "/Game/FirstPerson/Audio/SpikeTrapAudio.SpikeTrapAudio" 1.0 1.0 0.0 0 0))))
    (:Finished
      (goto _label Reset))))

(fn ConstructionScript
  (|CallParentFunction))

(fn TriggerTrap
  (params (TriggeringPawn :type Pawn%20Object%20Reference))
  (CallFunction|StartTimeline))