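; BP_ItemParentClass is a base actor for interactable, collectable items.
; Entering interact range creates a screen-space prompt widget for that player, attached to the component from GetInteractComponent, and exiting destroys it.
; OnCollect looks up DT_Collectables by the ItemType enum name, then destroys the actor and returns type, description and a zero amount.
; Interact returns only default values, and the getters supply the prompt text and root attachment point.
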(event EventOnInteractRangeEnter
  (params (InteractingPlayer :type BP%20Player%20Character%20Object%20Reference))
  ;[1 1 1] Create widget for the calling player
  (Variables|Default|GetTemporaryWidgetComponent
    (:then)
    (:else
      (bind _returnvalue (UserInterface|CreateWidget "/Game/_PURSUER/Widget_Blueprints/WBP_InteractWidget.WBP_InteractWidget_C" (.AsPlayer%20Controller (Utilities|Casting|CastToPlayerController (Pawn|GetController InteractingPlayer))) (CallFunction|GetInteractText)))
      (bind _returnvalue_2 (AddComponent|AddWidgetComponent false))
      (bind _output_get (Variables|Default|SetTemporaryWidgetComponent _returnvalue_2))
      (UserInterface|SetWidget _output_get _returnvalue)
      (Class|WidgetComponent|SetWidgetSpace _output_get "Screen")
      (Class|WidgetComponent|SetDrawatDesiredSize _output_get true)
      (Collision|SetCollisionEnabled _output_get "NoCollision")
      (Transformation|AttachComponentToComponent _output_get (CallFunction|GetInteractComponent) "None" "SnapToTarget" "SnapToTarget" "SnapToTarget" true))))

(event EventOnInteractRangeExit
  ;[1 1 1] Destroy the widget component on this BP_Item
  (bind _temporarywidgetcomponent (Variables|Default|GetTemporaryWidgetComponent)
    (:then
      (Components|DestroyComponent _temporarywidgetcomponent))
    (:else)))

(fn ConstructionScript)

(fn GetInteractText
  (return (Variables|Default|GetInteractText)))

(fn GetInteractComponent
  (return (Variables|Default|GetDefaultSceneRoot)))

(fn Interact
  (return "NewEnumerator0" 0))

(fn OnCollect
  (bind _returnvalue (Utilities|GetDataTableRow "/Game/_PURSUER/DataTables/DT_Collectables.DT_Collectables" (Utilities|String|StringToName (Utilities|String|EnumtoString (Variables|Default|GetItemType))))
    (:then
      (Actor|DestroyActor)
      (return (.CollectableType (Utilities|Struct|BreakStruct_Collectable _returnvalue)) (.Description (Utilities|Struct|BreakStruct_Collectable _returnvalue)) 0))))